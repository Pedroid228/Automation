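; Testable inventory item actor showing a sphere, cube or cylinder mesh with its score as floating text.
; The construction script picks the mesh from ItemType, creates a dynamic material and applies random colors to mesh and text.
; Set_Inventory_Data_Event overrides type, score and color, then refreshes the mesh, material and text.
; Tick yaws the text to face the player pawn.
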(event Custom|Set_Inventory_Data_Event
  (params (item_type :type EInventory_Item_Types%20Enum :default "Sphere") (score :type Integer) (color :type Linear%20Color%20Structure))
  (Variables|Default|SetItem_Type item_type)
  (Variables|Default|SetScore score)
  (Variables|Default|SetNew_Color color)
  (CallFunction|SetStaticMesh (Variables|Default|GetItem_Type))
  (Rendering|Material|SetVectorParameterValue (Variables|Default|GetMDI_Material) "Color" (Variables|Default|GetNew_Color) :!class /Script/Engine.MaterialInstanceDynamic)
  (CallFunction|UpdateTextRender (Math|Conversions|ToColor(LinearColor) (Variables|Default|GetNew_Color))))

(event EventBeginPlay)

(event Collision|EventActorBeginOverlap
  (params (OtherActor :type Actor%20Object%20Reference)))

(event EventTick
  (params (DeltaSeconds :type Float%20%28single-precision%29))
  (bind _text_render (Variables|Default|GetText_Render))
  (bind _returnvalue (Transformation|GetWorldRotation _text_render))
  (bind (_roll _pitch) (Math|Rotator|BreakRotator _returnvalue))
  (Transformation|SetWorldRotation (Variables|Default|GetText_Render) (Math|Rotator|MakeRotator _roll _pitch (.Yaw (Math|Rotator|BreakRotator (Math|Rotator|FindLookatRotation (Transformation|GetWorldLocation (Variables|Default|GetText_Render)) (Transformation|GetActorLocation (Game|Player|GetPlayerPawn 0)))))) false false))

(fn ConstructionScript
  (bind _returnvalue (Math|Random|RandomFloat))
  (bind _returnvalue_2 (Math|Random|RandomFloat))
  (bind _returnvalue_3 (Math|Random|RandomFloat))
  (bind _linearcolor (Utilities|Struct|MakeLinearColor _returnvalue_2 _returnvalue_3 _returnvalue 1.0))
  (CallFunction|SetStaticMesh (Variables|Default|GetItem_Type))
  (bind _returnvalue_4 (Rendering|Material|CreateDynamicMaterialInstance (Variables|Character|GetMesh) 0 "/Game/Automation/Materials/M_Item_Base.M_Item_Base" "None" :!class /Script/Engine.PrimitiveComponent))
  (bind _output_get (Variables|Default|SetMDI_Material _returnvalue_4))
  (Rendering|Material|SetVectorParameterValue _output_get "Color" _linearcolor :!class /Script/Engine.MaterialInstanceDynamic)
  (CallFunction|UpdateTextRender (Math|Conversions|ToColor(LinearColor) _linearcolor)))

(fn SetStaticMesh
  (params (new_item_type :type EInventory_Item_Types%20Enum :default "Sphere"))
  (Components|StaticMesh|SetStaticMesh (Variables|Character|GetMesh) (Utilities|Select :Index new_item_type :Sphere "/Game/StarterContent/Shapes/Shape_Sphere.Shape_Sphere" :Cube "/Game/StarterContent/Shapes/Shape_Cube.Shape_Cube" :Cylinder "/Game/StarterContent/Shapes/Shape_Cylinder.Shape_Cylinder")))

(fn UpdateTextRender
  (params (new_color :type Color%20Structure))
  (Rendering|Components|TextRender|SetTextRenderColor (Variables|Default|GetText_Render) new_color)
  (Rendering|Components|TextRender|SetText (Variables|Default|GetText_Render) (Utilities|Text|ToText(Integer) (Variables|Default|GetScore))))